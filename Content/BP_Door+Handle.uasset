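; Interactable door that opens once when the Interact input is pressed while its trigger box has enabled input.
; Box overlap begin and end toggle input for player controller 0, without checking which actor overlaps.
; A single timeline rolls the handle and slides the gate along Z, and a 2D chime plays after a short delay.
; The DoOnce is never reset, so the door has no closing path.
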(event `self.Box_coll.OnComponentBeginOverlap`
  (params (OverlappedComponent :type "PrimitiveComponent Object Reference") (OtherActor :type "Actor Object Reference") (OtherComp :type "PrimitiveComponent Object Reference") (OtherBodyIndex :type Integer) (bFromSweep :type Boolean) (SweepResult :type "HitResult Structure (by ref)"))
  (`self.EnableInput` (`GameplayStatics.GetPlayerController` 0)))

(event `self.Box_coll.OnComponentEndOverlap`
  (params (OverlappedComponent :type "PrimitiveComponent Object Reference") (OtherActor :type "Actor Object Reference") (OtherComp :type "PrimitiveComponent Object Reference") (OtherBodyIndex :type Integer))
  (`self.DisableInput` (`GameplayStatics.GetPlayerController` 0)))

(event `InputAction|Interact`
  (params (Key :type "Key Structure"))
  ;[0 0.2737 1] when the character interact, the handle will make an animation as well as the door.
  (:`Pressed`
    (`/Engine/EditorBlueprintResources/StandardMacros.DoOnce` false
      (:`Completed`
        (`|ExecutionSequence`
          (:`then_0`
            (bind (_direction _handlerotate _doorslide) (`Timeline|Timeline`)
              (:`Update`
                (`SceneComponent.K2_SetRelativeRotation` (`self.handle`) (`KismetMathLibrary.MakeRotator` _handlerotate) false false)
                (`SceneComponent.K2_SetRelativeLocation` (`self.gate`) (`KismetMathLibrary.MakeVector` 5.0 -200.0 _doorslide) false false))))
          (:`then_1`
            (`KismetSystemLibrary.Delay` 1.5)
            (`GameplayStatics.PlaySound2D` "/Game/EpicPlatformer/SFX/SFX_Chime_01A.SFX_Chime_01A" 1.0 1.0 0.0 null null)))))))

(fn `UserConstructionScript`)