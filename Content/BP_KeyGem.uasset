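; BP_KeyGem is a spinning key gem pickup that adds to the player character's key count.
; Tick yaws the gem a fixed step per frame, independent of delta time.
; Any Box overlap plays a chime, then adds K to player 0's CharacterBP Key and destroys the gem, without checking the overlapping actor.
; On BeginPlay, each gem creates its own CoinScreen counter widget on the viewport.
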(event `self.ReceiveTick`
  (params (DeltaSeconds :type "Float (single-precision)"))
  (bind _keygem (`self.KeyGem`))
  (bind (_relativerotation_roll _relativerotation_pitch _relativerotation_yaw) (`KismetMathLibrary.BreakRotator` (`SceneComponent.RelativeRotation` _keygem)))
  ;[1 0.9867 0.1699] Key Rotation
  (`SceneComponent.K2_SetRelativeRotation` _keygem (`KismetMathLibrary.MakeRotator` _relativerotation_roll _relativerotation_pitch (+ _relativerotation_yaw 1.0)) false false))

(event `self.box.OnComponentBeginOverlap`
  (params (OverlappedComponent :type "PrimitiveComponent Object Reference") (OtherActor :type "Actor Object Reference") (OtherComp :type "PrimitiveComponent Object Reference") (OtherBodyIndex :type Integer) (bFromSweep :type Boolean) (SweepResult :type "HitResult Structure (by ref)"))
  ;[0 0.6897 1] for every Key, when the character overlaps, the Key makes a sound then disappear.
  (`GameplayStatics.PlaySound2D` "/Game/EpicPlatformer/SFX/SFX_Chime_06B.SFX_Chime_06B" 1.0 1.0 0.0 null null)
  (bind _ascharacter_bp (cast `/Game/EpicPlatformer/Character/CharacterBP` (`GameplayStatics.GetPlayerPawn` 0)))
  (set `/Game/EpicPlatformer/Character/CharacterBP.Key` (+ (`/Game/EpicPlatformer/Character/CharacterBP.Key` _ascharacter_bp) (`self.k`)) _ascharacter_bp)
  (`self.K2_DestroyActor`))

(event `self.ReceiveBeginPlay`
  ;[1 0.9546 0.8183] event to show the coin counter screen
  (bind _returnvalue (`|CreateWidget` "/Game/CoinScreen.CoinScreen_C"))
  (`UserWidget.AddToViewport` _returnvalue 0))

(fn `UserConstructionScript`)