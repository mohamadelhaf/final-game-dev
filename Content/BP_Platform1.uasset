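; Moving platform actor that slides its static mesh between two relative locations, LocationA and LocationB.
; The MovePlatform1 event plays the PlatformAnimation timeline, whose Location track drives a vector lerp on each update without sweeping.
; StopPlatform1 halts the timeline in place.
; The construction script sets the timeline's play rate from the Speed variable.
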(event `MovePlatform1`
  (bind (_direction _location) (`Timeline|PlatformAnimation` :!label _label)
    (:`Update`
      (`SceneComponent.K2_SetRelativeLocation` (`self.StaticMesh`) (`KismetMathLibrary.VLerp` (`self.Location A`) (`self.Location B`) _location) false false))))

(event `StopPlatform1`
  (goto _label :!via `Stop`))

(fn `UserConstructionScript`
  (`TimelineComponent.SetPlayRate` (`self.PlatformAnimation`) (`self.Speed`)))