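; BP_PowerUp is a gem pickup that spins in place and disappears when its box is overlapped.
; Tick advances the PowerUp component's yaw by a fixed step each frame, independent of delta time.
; Any overlap plays a chime, then casts the player pawn to CharacterBP without checking the overlapping actor.
; On success, it reassigns the character's PowerUp to its current value, destroys itself and prints the Print text.
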(event `self.ReceiveTick`
  (params (DeltaSeconds :type "Float (single-precision)"))
  (bind _powerup (`self.PowerUp`))
  (bind (_relativerotation_roll _relativerotation_pitch _relativerotation_yaw) (`KismetMathLibrary.BreakRotator` (`SceneComponent.RelativeRotation` _powerup)))
  ;[1 0.9867 0.1699] Gem Rotation
  (`SceneComponent.K2_SetRelativeRotation` _powerup (`KismetMathLibrary.MakeRotator` _relativerotation_roll _relativerotation_pitch (+ _relativerotation_yaw 1.0)) false false))

(event `self.box.OnComponentBeginOverlap`
  (params (OverlappedComponent :type "PrimitiveComponent Object Reference") (OtherActor :type "Actor Object Reference") (OtherComp :type "PrimitiveComponent Object Reference") (OtherBodyIndex :type Integer) (bFromSweep :type Boolean) (SweepResult :type "HitResult Structure (by ref)"))
  ;[0 0.6897 1] for every Gem, when the character overlaps, the gem makes a sound then disappear, and print: POWER UP!
  (`GameplayStatics.PlaySound2D` "/Game/EpicPlatformer/SFX/SFX_Chime_05B.SFX_Chime_05B" 1.0 1.0 0.0 null null)
  (bind _ascharacter_bp (cast `/Game/EpicPlatformer/Character/CharacterBP` (`GameplayStatics.GetPlayerPawn` 0)))
  (set `/Game/EpicPlatformer/Character/CharacterBP.power up` (`/Game/EpicPlatformer/Character/CharacterBP.power up` _ascharacter_bp) _ascharacter_bp)
  (`self.K2_DestroyActor`)
  (`KismetSystemLibrary.PrintText` (`KismetTextLibrary.Conv_StringToText` (`KismetStringLibrary.Concat_StrStr` "                                                                                                                                                                                                                                             " (`self.print`)))))

(fn `UserConstructionScript`)