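; BP_Button is a pressure button that responds when the player character (CharacterBP) or a BP_Ball overlaps its sphere trigger.
; Pressing swaps the button's material to the pressed (green) one and plays the ButtonPress timeline, which lerps its relative Z toward ActivatedPosition.
; Any end overlap, regardless of actor, restores the blue material and reverses the timeline.
; A ResetButton event sets the timeline's time.
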(event `self.Sphere.OnComponentBeginOverlap`
  (params (OverlappedComponent :type "PrimitiveComponent Object Reference") (OtherActor :type "Actor Object Reference") (OtherComp :type "PrimitiveComponent Object Reference") (OtherBodyIndex :type Integer) (bFromSweep :type Boolean) (SweepResult :type "HitResult Structure (by ref)"))
  (`|ExecutionSequence`
    (:`then_0`
      (cast `/Game/EpicPlatformer/Character/CharacterBP` OtherActor))
    (:`then_1`
      (cast `/Game/BP_Ball` OtherActor)))
  (`self.ButtonPressed`))

(event `self.Sphere.OnComponentEndOverlap`
  (params (OverlappedComponent :type "PrimitiveComponent Object Reference") (OtherActor :type "Actor Object Reference") (OtherComp :type "PrimitiveComponent Object Reference") (OtherBodyIndex :type Integer))
  (`self.ButtonReleased`))

(event `ButtonPressed`
  ;[0 1 0.1909] When the button is Pressed, set the color to green
  (`PrimitiveComponent.CreateDynamicMaterialInstance` (`self.Button`) 0 "/Game/Button.Button" "None")
  (`PrimitiveComponent.SetMaterial` (`self.Button`) 0 "/Game/EpicPlatformer/Meshes/Props/Buttons/Button_A/Material/M_Button_A_2.M_Button_A_2")
  ;[1 1 1] Animation for the button
  (`TimelineComponent.SetPlayRate` (`self.ButtonPress`) 2.0)
  (bind (_direction _basic) (`Timeline|ButtonPress` :!label _label)
    (:`Update`
      (`SceneComponent.K2_SetRelativeLocation` (`self.Button`) (`KismetMathLibrary.MakeVector` 0.0 0.0 (`KismetMathLibrary.Lerp` 0.0 (`self.ActivatedPosition`) _basic)) false false))))

(event `ResetButton`
  (params (Target :type "MaterialInstanceDynamic Object Reference"))
  ;[1 1 1] Animation for the button
  (goto _label :!via `SetNewTime`))

(event `ButtonReleased`
  ;[1 1 1] When Button is released, make the color blue
  (`PrimitiveComponent.SetMaterial` (`self.Button`) 0 "/Game/EpicPlatformer/Meshes/Props/Buttons/Button_A/Material/M_Button_A.M_Button_A")
  (goto _label :!via `Reverse`))

(fn `UserConstructionScript`)